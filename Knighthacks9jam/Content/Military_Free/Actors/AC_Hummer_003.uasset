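; Hummer actor that acts as the win trigger when the first-person player character enters its Box.
; On overlap it checks the character's six item flags, covering survival supplies, gear and documents.
; With all items, it disables input, blends the view to itself, hides the character and calls ShowVictory on PlayerScreensComponent.
; Otherwise that component shows a timed message, whose text is currently the component reference converted to text.
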(event `self.Box.OnComponentBeginOverlap`
  (params (OverlappedComponent :type "PrimitiveComponent Object Reference") (OtherActor :type "Actor Object Reference") (OtherComp :type "PrimitiveComponent Object Reference") (OtherBodyIndex :type Integer) (bFromSweep :type Boolean) (SweepResult :type "HitResult Structure (by ref)"))
  (bind _returnvalue (`GameplayStatics.GetPlayerController` 0))
  (bind _asbp_first_person_character (cast `/Game/FirstPerson/Blueprints/BP_FirstPersonCharacter` OtherActor))
  (if (and (`/Game/FirstPerson/Blueprints/BP_FirstPersonCharacter.HasWater` _asbp_first_person_character) (`/Game/FirstPerson/Blueprints/BP_FirstPersonCharacter.HasFood` _asbp_first_person_character) (`/Game/FirstPerson/Blueprints/BP_FirstPersonCharacter.HasFirstAid` _asbp_first_person_character) (`/Game/FirstPerson/Blueprints/BP_FirstPersonCharacter.HasRadio` _asbp_first_person_character) (`/Game/FirstPerson/Blueprints/BP_FirstPersonCharacter.HasFlashlight` _asbp_first_person_character) (`/Game/FirstPerson/Blueprints/BP_FirstPersonCharacter.HasDocuments` _asbp_first_person_character))
    (`self.DisableInput` _asbp_first_person_character _returnvalue)
    (`PlayerController.SetViewTargetWithBlend` _returnvalue self 0.0 "VTBlend_Linear" 0.0 false)
    (`self.SetActorHiddenInGame` _asbp_first_person_character true)
    (`PlayerScreensComponent.ShowVictory` (`self.GetComponentByClass` _asbp_first_person_character "/Script/Knighthacks9jam.PlayerScreensComponent") 5.0)
    (else
      (bind _returnvalue_2 (`self.GetComponentByClass` _asbp_first_person_character "/Script/Knighthacks9jam.PlayerScreensComponent"))
      (`PlayerScreensComponent.ShowMessage` _returnvalue_2 (`KismetTextLibrary.Conv_ObjectToText` _returnvalue_2) 3.0))))

(fn `UserConstructionScript`)